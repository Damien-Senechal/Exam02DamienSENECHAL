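; Enemy Blueprint that chases the player's BP_Mage and attacks it at close range.
; A looping FollowPlayer event re-issues AI MoveTo or triggers Attack by distance, re-checking after delays until dead.
; DoOnce gates with timed resets throttle outgoing and incoming damage, pulsing IsAttacking and TakeHit flags.
; Depleted health sets Dead, ending the loop and leaving the damage gate closed.
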(event Custom|FollowPlayer
  (if (not (Variables|Default|GetDead))
    (if (>= (Transformation|GetDistanceTo (Variables|Default|GetPlayerRef)) 3e+02)
      (AI|AIMoveTo self "0, 0, 0" (Variables|Default|GetPlayerRef) 5.0 false
        (:then
          (Utilities|FlowControl|Delay 5.0)))
      (else
        (CallFunction|Attack)
        (Utilities|FlowControl|Delay 1.0)))
    (CallFunction|FollowPlayer)))

(event Custom|Attack
  (Utilities|FlowControl|DoOnce false :!label _label
    (:Completed
      (Game|Damage|ApplyDamage (Variables|Default|GetPlayerRef) 1.0 0 0)
      (Variables|Default|SetIsAttacking true)
      (Utilities|FlowControl|Delay 1.0)
      (Variables|Default|SetIsAttacking false)
      (goto _label Reset))))

(event EventBeginPlay
  (bind _asbp_mage (Utilities|Casting|CastToBP_Mage (Game|GetPlayerCharacter 0)))
  (Variables|Default|SetPlayerRef _asbp_mage)
  (CallFunction|FollowPlayer))

(event Game|Damage|EventAnyDamage
  (params (Damage :type Float%20%28single-precision%29) (DamageType :type Damage%20Type%20Object%20Reference) (InstigatedBy :type Controller%20Object%20Reference) (DamageCauser :type Actor%20Object%20Reference))
  (Utilities|FlowControl|DoOnce false :!label _label
    (:Completed
      (bind _output_get (Variables|Default|SetHealth (- (Variables|Default|GetHealth) Damage)))
      (if (<= _output_get 0.0)
        (Variables|Default|SetDead true)
        (else
          (Variables|Default|SetTakeHit true)
          (Utilities|FlowControl|Delay 1.0)
          (Variables|Default|SetTakeHit false)
          (goto _label Reset))))))

(fn ConstructionScript)